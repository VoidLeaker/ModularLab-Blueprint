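; BP_InteractDoor is an interactable door that swings open and closed by rotating around its yaw axis.
; The Interactable event checks an IsOpen flag and calls OpenDoor or ClosedDoor, which play or reverse a single timeline.
; The timeline's Sliding track drives the Door component's relative rotation on each update.
; On BeginPlay the door also runs one delayed open and close cycle automatically.
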(event Custom|ClosedDoor
  (Variables|Default|SetisOpen false)
  (bind _sliding (Timeline|DoorTimeline Reverse)
    (:Update
      (Transformation|SetRelativeRotation (Variables|Default|GetDoor) (Math|Rotator|MakeRotator 0.0 0.0 _sliding) false false))))

(event Custom|OpenDoor
  (Variables|Default|SetisOpen true)
  (bind _sliding (Timeline|DoorTimeline Play)
    (:Update
      (Transformation|SetRelativeRotation (Variables|Default|GetDoor) (Math|Rotator|MakeRotator 0.0 0.0 _sliding) false false))))

(event EventBeginPlay
  (Utilities|FlowControl|Delay 1.0)
  (CallFunction|OpenDoor)
  (Utilities|FlowControl|Delay 1.0)
  (CallFunction|ClosedDoor))

(event EventInteractable
  (params (Interactor :type Actor%20Object%20Reference))
  (if (Variables|Default|GetisOpen)
    (CallFunction|ClosedDoor)
    (else
      (CallFunction|OpenDoor))))

(fn ConstructionScript)