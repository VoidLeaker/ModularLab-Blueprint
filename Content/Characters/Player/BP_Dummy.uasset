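; BP_Dummy is a player character with Enhanced Input movement, jumping, looking and a teleport event.
; BeginPlay applies IMC_PlayerInput through EasyMappingContext; the move action feeds a Movement function that derives directions from control rotation, ignoring pitch.
; Jump and look actions drive the built-in jump and controller yaw/pitch functions.
; Teleport looks up a BP_TeleporterExit by class and places the character at its box collider's location.
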(event Custom|Teleport
  (bind _returnvalue (Actor|GetActorOfClass "/Game/Blueprints/Teleporter/BP_Teleporter-Exit.BP_Teleporter-Exit_C"))
  (Transformation|SetActorLocation (Transformation|GetWorldLocation (Variables|/Game/Blueprints/Teleporter/BP_Teleporter-Exit.BP_Teleporter-Exit_C|GetBoxCollider _returnvalue)) false false))

(event Input|EnhancedActionEvents|EnhancedInputActionIA_Look
  (params (ActionValue :type Vector%202D%20Structure) (ElapsedSeconds :type Float%20%28double-precision%29) (TriggeredSeconds :type Float%20%28double-precision%29) (InputAction :type Input%20Action%20Object%20Reference :default "/Game/Characters/Input/InputAction/IA_Look.IA_Look"))
  ;[0.15 0.15 0.15 0.5] Character Movement System
  (Pawn|Input|AddControllerYawInput (.x ActionValue))
  (Pawn|Input|AddControllerPitchInput (.y ActionValue)))

(event Input|EnhancedActionEvents|EnhancedInputActionIA_Move
  (params (ActionValue :type Vector%202D%20Structure) (ElapsedSeconds :type Float%20%28double-precision%29) (TriggeredSeconds :type Float%20%28double-precision%29) (InputAction :type Input%20Action%20Object%20Reference :default "/Game/Characters/Input/InputAction/IA_Move.IA_Move"))
  ;[0.15 0.15 0.15 0.5] Character Movement System
  (|Movement (.x ActionValue) (.y ActionValue)))

(event Input|EnhancedActionEvents|EnhancedInputActionIA_Jump
  (params (ActionValue :type Boolean) (ElapsedSeconds :type Float%20%28double-precision%29) (TriggeredSeconds :type Float%20%28double-precision%29) (InputAction :type Input%20Action%20Object%20Reference :default "/Game/Characters/Input/InputAction/IA_Jump.IA_Jump"))
  ;[0.15 0.15 0.15 0.5] Character Movement System
  (:Started
    (Character|Jump))
  (:Completed
    (Character|StopJumping)))

(event EventBeginPlay
  ;[0.15 0.15 0.15 0.5] Character Movement System
  (CallFunction|EasyMappingContext "/Game/Characters/Input/IMC_PlayerInput.IMC_PlayerInput"))

(fn ConstructionScript)